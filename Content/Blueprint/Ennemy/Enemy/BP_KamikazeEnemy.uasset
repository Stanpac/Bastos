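; Kamikaze enemy that blows itself up to damage nearby player characters.
; StartExplosion fires once, adds a movement-stopped gameplay tag and plays a montage, calling TriggerExplosion on completion.
; TriggerExplosion starts death without the death montage, damages players found by a sphere overlap and spawns a Niagara effect.
; The node scaling that effect to the explosion range is disconnected.
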(event `StartExplosion`
  (if (not (`self.IsExploding`))
    (set `self.IsExploding` true)
    (`GameplayTagCountContainerInterface.UpdateTagCount` (struct :`TagName` "Gameplay.MovementStopped") 1)
    (`|PlayMontage` (`self.Mesh`) (`self.ExplosionMontage`)
      (:`OnCompleted`
        (`self.TriggerExplosion`)))))

(event `TriggerExplosion`
  (set `self.UseDeathMontage` false)
  (bind _outactors (`KismetSystemLibrary.SphereOverlapActors` (`self.K2_GetActorLocation`) (`self.ExplosionRange`) (`|MakeArray` "ObjectTypeQuery3" :!type "EObjectTypeQuery Enum") "/Script/Pac.PacPlayerCharacter"))
  (`PacHealthComponent.StartDeath` (`self.HealthComponent`))
  (for _array_element _outactors
    (bind _aspac_player_character (cast `PacPlayerCharacter` _array_element))
    (`PacHealthComponent.TakeDamage` (`PacCharacter.HealthComponent` _aspac_player_character) (`self.ExplosionDamage`) self))
  (bind _returnvalue (`NiagaraFunctionLibrary.SpawnSystemAtLocation` (`self.ExpolosionVFX`) (`self.K2_GetActorLocation`) (struct) (1.0 1.0 1.0) true true "AutoRelease")))

(fn `UserConstructionScript`)