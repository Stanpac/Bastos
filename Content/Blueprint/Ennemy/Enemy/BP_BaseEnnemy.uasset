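; Base enemy character Blueprint that handles combat feedback and links health, AI and an overhead status widget.
; A camera-facing W_EnemyWidget shows spotted and charging states, with charging also driving a timed VFX.
; Fire and reload play montages, respectively ending the charge and halting movement.
; Health component events trigger hit and death feedback, with hits reported to AI damage sensing, while aggro reset forwards to AIC_BaseEnnemy.
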(event `self.ReceiveTick`
  (params (DeltaSeconds :type "Float (single-precision)"))
  (`SceneComponent.K2_SetWorldRotation` (`self.Widget`) (`KismetMathLibrary.FindLookAtRotation` (`SceneComponent.K2_GetComponentLocation` (`self.Widget`)) (`Controller.GetPlayerViewPoint` (`GameplayStatics.GetPlayerController` 0))) false false))

(event `self.ReceiveBeginPlay`
  (bind _asw_enemy_widget (cast `/Game/UI/Character/W_EnemyWidget` (`WidgetComponent.GetWidget` (`self.Widget`))))
  (`/Game/UI/Character/W_EnemyWidget.Initialize` _asw_enemy_widget self))

(event `self.K2_Fire`
  (`|PlayMontage` (`self.Mesh`) (`self.Shoot Montage`)
    (:`then`
      (`self.Stop Charging`))))

(event `self.K2_Reload`
  (`|PlayMontage` (`self.Mesh`) (`self.Reload Montage`)
    (:`then`
      (`NavMovementInterface.StopActiveMovement` (`self.CharacterMovement`)))))

(event `self.HealthComponent.OnTakeDamage`
  (params (HealthComponent :type "PacHealthComponent Object Reference") (OldValue :type Integer) (NewValue :type Integer) (Instigator :type "Actor Object Reference"))
  (`AISense_Damage.ReportDamageEvent` self Instigator 0.0 (`self.K2_GetActorLocation`))
  (`|PlayMontage` (`self.Mesh`) (`self.Hit Montage`) 1.0 0.0 "None" false
    (:`then`
      (`GameplayStatics.PlaySoundAtLocation` "/Game/SoundDesign/Enemy_Sounds/EnemyHit_Input.EnemyHit_Input" (`self.K2_GetActorLocation`) (struct) 1.0 1.0 0.0 null null null null))))

(event `AggroTriger`
  (bind _asw_enemy_widget (cast `/Game/UI/Character/W_EnemyWidget` (`WidgetComponent.GetWidget` (`self.Widget`))))
  (`/Game/UI/Character/W_EnemyWidget.Enemy Spotted ` _asw_enemy_widget))

(event `self.HealthComponent.OnDeath`
  (`GameplayStatics.PlaySoundAtLocation` "/Game/SoundDesign/Enemy_Sounds/EnemyDeath_Input.EnemyDeath_Input" (`self.K2_GetActorLocation`) (struct) 1.0 1.0 0.0 null null null null))

(event `StartCharging`
  (if (not (and (`self.Charging`) (not (`GameplayTagAssetInterface.HasMatchingGameplayTag` (struct :`TagName` "Gameplay.PreventFromShooting")))))
    (set `self.Charging` true)
    (bind _asw_enemy_widget (cast `/Game/UI/Character/W_EnemyWidget` (`WidgetComponent.GetWidget` (`self.Widget`))))
    (`/Game/UI/Character/W_EnemyWidget.Charging` _asw_enemy_widget)
    (`ActorComponent.Activate` (`self.ChargingVfx`) true)
    (`NiagaraComponent.SetVariableFloat` (`self.ChargingVfx`) "ChargingTime" (`self.ChargingTime`))
    (`NiagaraComponent.SetVariableFloat` (`self.ChargingVfx`) "ChargingTime" (`self.ChargingTime`))))

(event `Stop Charging`
  (set `self.Charging` false)
  (bind _asw_enemy_widget (cast `/Game/UI/Character/W_EnemyWidget` (`WidgetComponent.GetWidget` (`self.Widget`))))
  (`/Game/UI/Character/W_EnemyWidget.Reset ` _asw_enemy_widget)
  (`ActorComponent.Deactivate` (`self.ChargingVfx`)))

(event `Reset Aggro`
  (bind _asaic_base_ennemy (cast `/Game/Blueprint/Ennemy/Enemy/AIC/AIC_BaseEnnemy` (`self.GetController`)))
  (`/Game/Blueprint/Ennemy/Enemy/AIC/AIC_BaseEnnemy.Reset Aggro` _asaic_base_ennemy))

(fn `UserConstructionScript`)