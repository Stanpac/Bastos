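; A stackable kamikaze effect that makes its owning character explode when the effect is removed with a trigger event.
; It spawns an explosion VFX at the owner's location and plays a 2D detonation sound.
; A sphere overlap finds other pawns within the kamikaze radius and damages their health components by damage per stack times stack count, crediting the owner as instigator.
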(event `self.K2_EffectRemove`
  (params (TriggerEvent :type Boolean))
  (bind _returnvalue (`PacEffectComponent.GetPacCharacterOwner` (`self.GetTargetEffectContainer`)))
  (if TriggerEvent
    (`self.SpawnVFXExplosion`)
    (bind _outactors (`KismetSystemLibrary.SphereOverlapActors` (`Actor.K2_GetActorLocation` _returnvalue) (`self.Kamikaze Radius`) (`self.Explosion Querry Type`) "/Script/Engine.Pawn" (`|MakeArray` _returnvalue :!type "Actor Object Reference")))
    (for _array_element _outactors
      (`PacHealthComponent.TakeDamage` (`Actor.GetComponentByClass` _array_element "/Script/Pac.PacHealthComponent") (* (`self.DamagePerStack`) (`self.StackCount`)) (`PacEffectComponent.GetPacCharacterOwner` (`self.GetTargetEffectContainer`))))))

(fn `SpawnVFXExplosion`
  (`NiagaraFunctionLibrary.SpawnSystemAtLocation` (`self.Explosion VFX`) (`Actor.K2_GetActorLocation` (`PacEffectComponent.GetPacCharacterOwner` (`self.GetTargetEffectContainer`))))
  (`GameplayStatics.PlaySound2D` "/Game/SoundDesign/Bullets/DetonationShot_Proc_Input.DetonationShot_Proc_Input" 1.0 1.0 0.0 null null))