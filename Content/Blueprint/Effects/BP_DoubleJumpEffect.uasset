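; Double-jump effect that reacts to the owning Pac character's extra jumps by using up stacks.
; It binds to the character's jumped event on apply and unbinds on remove.
; A jump past the first removes one stack, spawns a pooled Niagara effect at the character and plays a 2D sound.
; Jumps made while the character has the coyote-time gameplay tag are ignored.
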(event `self.K2_EffectApply`
  (add `PacCharacter.OnJumpedEvent` (`PacEffectComponent.GetPacCharacterOwner` (`self.GetTargetEffectContainer`)) (delegate `OnJumpedEvent_Event`)))

(event `OnJumpedEvent_Event`
  (bind _returnvalue (`PacEffectComponent.GetPacCharacterOwner` (`self.GetTargetEffectContainer`)))
  (if (and (> (`Character.JumpCurrentCount` _returnvalue) 1) (not (`GameplayTagAssetInterface.HasMatchingGameplayTag` _returnvalue (struct :`TagName` "Gameplay.CoyoteTime"))))
    (`self.TryModifyStackValue` -1)
    (`NiagaraFunctionLibrary.SpawnSystemAtLocation` (`self.Jump Vfx`) (`Actor.K2_GetActorLocation` (`PacEffectComponent.GetPacCharacterOwner` (`self.GetTargetEffectContainer`))) (struct) (1.0 1.0 1.0) true true "AutoRelease")
    (`GameplayStatics.PlaySound2D` "/Game/SoundDesign/Bullets/JumpShot_Jump_Input.JumpShot_Jump_Input" 1.0 1.0 0.0 null null)))

(event `self.K2_EffectRemove`
  (params (TriggerEvent :type Boolean))
  (remove `PacCharacter.OnJumpedEvent` (`PacEffectComponent.GetPacCharacterOwner` (`self.GetTargetEffectContainer`)) (`|CreateDelegate` :!event `OnJumpedEvent_Event`)))