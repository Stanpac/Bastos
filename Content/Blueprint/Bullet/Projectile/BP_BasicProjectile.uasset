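; BP_BasicProjectile is a projectile that damages the player character, with an impact effect named for enemy attacks.
; On overlap, actors matching ActorClassToIgnore are skipped; any other actor triggers ProjectileHit, and a PacPlayerCharacter first takes damage through its HealthComponent.
; A blocking hit spawns a pooled Niagara impact at the hit location, then calls ProjectileHit without applying damage.
; ActorToIgnore returns true for actors that are not ignored, despite its name.
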(event `self.CollisionComponent.OnComponentBeginOverlap`
  (params (OverlappedComponent :type "PrimitiveComponent Object Reference") (OtherActor :type "Actor Object Reference") (OtherComp :type "PrimitiveComponent Object Reference") (OtherBodyIndex :type Integer) (bFromSweep :type Boolean) (SweepResult :type "HitResult Structure (by ref)"))
  (bind _notignored (`self.ActorToIgnore` OtherActor))
  (if _notignored
    (bind _aspac_player_character (cast `PacPlayerCharacter` OtherActor)
      (:`then`
        (`PacHealthComponent.TakeDamage` (`PacCharacter.HealthComponent` _aspac_player_character) (`self.Damage`) (`self.GetInstigator`)))
      (:`CastFailed`
        _))
    (`self.ProjectileHit` OtherActor)))

(event `self.CollisionComponent.OnComponentHit`
  (params (HitComponent :type "PrimitiveComponent Object Reference") (OtherActor :type "Actor Object Reference") (OtherComp :type "PrimitiveComponent Object Reference") (NormalImpulse :type "Vector Structure") (Hit :type "HitResult Structure (by ref)"))
  (`NiagaraFunctionLibrary.SpawnSystemAtLocation` "/Game/VFX/NS_EnemyAttackImpact.NS_EnemyAttackImpact" (`.Location` (`GameplayStatics.BreakHitResult` Hit)) (struct) (1.0 1.0 1.0) true true "AutoRelease")
  (`self.ProjectileHit` OtherActor))

(fn `ActorToIgnore`
  (params (Actor :type "Actor Object Reference"))
  (returns (NotIgnored :type Boolean))
  (for _array_element (`self.ActorClassToIgnore`)
    (if (`GameplayStatics.ObjectIsA` Actor _array_element)
      (return false)))
  (return true))

(fn `UserConstructionScript`)