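; Propulsion bullet Blueprint that knocks characters away from its impact point and launches a directly hit character upward.
; On a blocking hit, it spawns a zone effect and sphere-overlaps nearby PacCharacters, excluding the hit actor.
; Async root motion pushes them radially, with a fixed lift if not falling and zeroed falling lateral friction, keeping velocity afterward.
; Players are moved too, but only non-player characters receive BP_PropulsionEffect.
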(event `self.OnTargetFound`
  (params (HitResult :type "HitResult Structure"))
  (bind (_bblockinghit _binitialoverlap _time _distance _location _impactpoint _normal _impactnormal _physmat _hitactor) (`GameplayStatics.BreakHitResult` HitResult))
  (`parent.OnTargetFound` HitResult)
  (if _bblockinghit
    (bind _actors__found (`self.GetActorsInSphere` _location _hitactor))
    (for _array_element _actors__found
      (bind _aspac_character (cast `PacCharacter` _array_element))
      (cast `PacPlayerCharacter` _aspac_character
        (:`then`
          _)
        (:`CastFailed`
          (`PacEffectComponent.TryAddOrUpdateEffect` (`PacCharacter.EffectComponent` _aspac_character) "/Game/Blueprint/Effects/BP_PropulsionEffect.BP_PropulsionEffect_C" 1)))
      (bind (_outcharactermovement _direction) (`self.CalculateDirection` _aspac_character _location))
      (set `CharacterMovementComponent.FallingLateralFriction` 0.0 _outcharactermovement)
      (`AsyncRootMovement.AsyncRootMovement` _outcharactermovement _direction (`self.ExpulsionStrength`) 0.0 false null "MaintainLastRootMotionVelocity"))
    (bind _aspac_character_2 (cast `PacCharacter` _hitactor))
    (cast `PacPlayerCharacter` _aspac_character_2
      (:`then`
        _)
      (:`CastFailed`
        (`PacEffectComponent.TryAddOrUpdateEffect` (`PacCharacter.EffectComponent` _aspac_character_2) "/Game/Blueprint/Effects/BP_PropulsionEffect.BP_PropulsionEffect_C" 1)))
    (`AsyncRootMovement.AsyncRootMovement` (`Character.CharacterMovement` _aspac_character_2) (`KismetMathLibrary.Vector_Up`) (`self.UpStrengthForHitTarget`) 0.0 false null "MaintainLastRootMotionVelocity")))

(fn `CalculateDirection`
  (params (PacCharacter :type "PacCharacter Object Reference") (From :type "Vector Structure"))
  (returns (OutCharacterMovement :type "CharacterMovementComponent Object Reference") (Direction :type "Vector Structure"))
  (bind _charactermovement (`Character.CharacterMovement` PacCharacter))
  (bind (_returnvalue_x _returnvalue_y _returnvalue_z) (`KismetMathLibrary.BreakVector` (`KismetMathLibrary.GetDirectionUnitVector` From (`Actor.K2_GetActorLocation` PacCharacter))))
  (`/Engine/EditorBlueprintResources/StandardMacros.IsValid` PacCharacter
    (:`Is Valid`
      (return _charactermovement (`KismetMathLibrary.MakeVector` _returnvalue_x _returnvalue_y (select `bool` (`|EnumInequality` (`CharacterMovementComponent.MovementMode` _charactermovement) "MOVE_Falling") :`false` _returnvalue_z :`true` 0.5))))))

(fn `GetActorsInSphere`
  (params (HitPos :type "Vector Structure") (HitActor :type "Actor Object Reference"))
  (returns (`Actors  Found` :type "Array of Actor Object Reference"))
  (`NiagaraFunctionLibrary.SpawnSystemAtLocation` (`self.ZonePropulsionFX`) HitPos (struct) (1.0 1.0 1.0) true true "None" false)
  (bind _outactors (`KismetSystemLibrary.SphereOverlapActors` (`local.HitPos`) (`self.Sphere Radius`) (`self.Object Types`) "/Script/Pac.PacCharacter" (`|MakeArray` (`local.HitActor`))))
  (return _outactors))