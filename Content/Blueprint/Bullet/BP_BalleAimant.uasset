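; BP_BalleAimant is a magnet bullet that pulls nearby characters toward its point of impact.
; On a blocking hit, it spawns a propulsion effect and sphere-overlaps for characters, excluding the player and the hit actor.
; Each has falling lateral friction zeroed, without restoring it here, and is launched on a suggested projectile arc scaled by a multiplier.
; A directly hit character is pushed upward with root motion, keeping its momentum afterward.
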(event `self.OnTargetFound`
  (params (HitResult :type "HitResult Structure"))
  (bind (_bblockinghit _binitialoverlap _time _distance _location _impactpoint _normal _impactnormal _physmat _hitactor) (`GameplayStatics.BreakHitResult` HitResult))
  (`parent.OnTargetFound` HitResult)
  (if _bblockinghit
    (`NiagaraFunctionLibrary.SpawnSystemAtLocation` (`self.ZonePropulsionFX`) _location (`KismetMathLibrary.MakeRotFromZ` _normal) (1.0 1.0 1.0) true true "None" false)
    (bind _outactors (`KismetSystemLibrary.SphereOverlapActors` _location (`self.Range`) (`self.Object Types`) "/Script/Pac.PacCharacter" (`|MakeArray` _hitactor)))
    (for _array_element _outactors
      (cast `PacPlayerCharacter` _array_element
        (:`CastFailed`
          (bind _aspac_character (cast `PacCharacter` _array_element))
          (set `CharacterMovementComponent.FallingLateralFriction` 0.0 (`Character.CharacterMovement` _aspac_character))
          (bind _outlaunchvelocity (`GameplayStatics.SuggestProjectileVelocity_CustomArc` (`Actor.K2_GetActorLocation` _aspac_character) _location))
          (`Character.LaunchCharacter` _aspac_character (* _outlaunchvelocity (`self.VelocityMultiplicator`)) true true))))
    (bind _aspac_character_2 (cast `PacCharacter` _hitactor))
    (`AsyncRootMovement.AsyncRootMovement` (`Character.CharacterMovement` _aspac_character_2) (`KismetMathLibrary.Vector_Up`) (`self.StrengthForHitTarget`) 0.0 false null "MaintainLastRootMotionVelocity")))