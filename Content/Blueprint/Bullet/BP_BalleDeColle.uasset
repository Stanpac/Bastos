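; BP_BalleDeColle is a bullet Blueprint that places a temporary actor where it hits a target.
; On target found, it runs the parent logic, then spawns its configured actor class at the hit location with the avatar character as instigator.
; After a short delay it binds to that PacCharacter's shoot event, so a later shot destroys the spawned actor and ends the bullet.
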(event `self.OnTargetFound`
  (params (HitResult :type "HitResult Structure"))
  (bind _returnvalue (`self.GetAvatarCharacter`))
  (`parent.OnTargetFound` HitResult)
  (bind _returnvalue_2 (`|SpawnActorFromClass` (`self.ActorClassToSpawn`) (`KismetMathLibrary.Conv_VectorToTransform` (`.Location` (`GameplayStatics.BreakHitResult` HitResult))) "AlwaysSpawn" "MultiplyWithRoot" null _returnvalue))
  (bind _aspac_character (cast `PacCharacter` _returnvalue))
  (`KismetSystemLibrary.Delay` 0.1)
  (add `PacCharacter.OnShoot` _aspac_character (delegate `OnShoot_Event`)))

(event `OnShoot_Event`
  (`Actor.K2_DestroyActor` (stale `self.OnTargetFound` _returnvalue_2))
  (`self.K2_EndBullet`))