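; Bullet Blueprint that, on activation, dashes its avatar character along the facing direction.
; It zeroes velocity, then runs a short additive async root-motion force with clamped exit velocity, ending the bullet on completion or failure.
; For player-controlled avatars, holding S with InputPreventFormDashing set skips the dash without calling EndBullet.
; Target hits pass straight to the parent class.
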(event `self.K2_ActivateBullet`
  (bind _returnvalue (`self.GetAvatarCharacter`))
  (bind _charactermovement (`Character.CharacterMovement` _returnvalue))
  (bind _asplayer_controller (cast `PlayerController` (`Pawn.GetController` (`self.GetAvatarCharacter`)))
    (:`then`
      (if (not (and (`PlayerController.IsInputKeyDown` _asplayer_controller "S") (`self.InputPreventFormDashing?`)))
        (set `MovementComponent.Velocity` (0.0 0.0 0.0) _charactermovement :!label _label)
        (`AsyncRootMovement.AsyncRootMovement` _charactermovement (`KismetMathLibrary.Normal` (`PacCharacter.GetFacingDirection` _returnvalue) 0.0) (`self.Launch Force`) 0.25 true null "ClampVelocity" (0.0 0.0 0.0) (`self.ClampVelocityOnFinish`)
          (:`OnComplete`
            _)
          (:`OnFail`
            (`KismetSystemLibrary.PrintString` "Dash fail")))
        (`self.K2_EndBullet`)))
    (:`CastFailed`
      (goto _label))))

(event `self.OnTargetFound`
  (params (HitResult :type "HitResult Structure"))
  (`parent.OnTargetFound` HitResult))