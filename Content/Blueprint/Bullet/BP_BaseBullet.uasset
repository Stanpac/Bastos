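; Base bullet Blueprint that resolves a shot's hit result into damage and visual feedback.
; On target found, it spawns a trail system from the avatar's feedback shoot transform to the impact point, or to the trace end on a miss.
; Blocking hits damage actors with a PacHealthComponent and spawn a damage effect.
; Other blocking hits spawn a ground impact effect and a temporary, randomly sized and rotated decal.
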(event `BulletTrail`
  (params (`Hit Result` :type "HitResult Structure"))
  (bind (_bblockinghit _binitialoverlap _time _distance _location _impactpoint _normal _impactnormal _physmat _hitactor _hitcomponent _hitbonename _bonename _hititem _elementindex _faceindex _tracestart _traceend) (`GameplayStatics.BreakHitResult` `Hit Result`))
  (`/Engine/EditorBlueprintResources/StandardMacros.IsValid` (`self.TrailSystem`)
    (:`Is Valid`
      (bind _aspac_character (cast `PacCharacter` (`self.GetAvatarCharacter`)))
      (bind (_returnvalue_location _returnvalue_rotation _returnvalue_scale) (`KismetMathLibrary.BreakTransform` (`PacCharacter.GetFeedBackShootTransForm` _aspac_character)))
      (bind _returnvalue (`NiagaraFunctionLibrary.SpawnSystemAtLocation` (`self.TrailSystem`) _returnvalue_location _returnvalue_rotation _returnvalue_scale true true "AutoRelease"))
      (`NiagaraComponent.SetVariableVec3` _returnvalue "VectorStart" _returnvalue_location)
      (`NiagaraComponent.SetVariableVec3` _returnvalue "VectorEnd" (select `bool` _bblockinghit :`false` _traceend :`true` _impactpoint)))))

(event `self.OnTargetFound`
  (params (HitResult :type "HitResult Structure"))
  (bind (_bblockinghit _binitialoverlap _time _distance _location _impactpoint _normal _impactnormal _physmat _hitactor) (`GameplayStatics.BreakHitResult` HitResult))
  (bind _returnvalue (`Actor.GetComponentByClass` _hitactor "/Script/Pac.PacHealthComponent"))
  (`self.BulletTrail` HitResult)
  (if _bblockinghit
    (`/Engine/EditorBlueprintResources/StandardMacros.IsValid` _returnvalue
      (:`Is Valid`
        (`self.Hit Healt Comp` HitResult _returnvalue))
      (:`Is Not Valid`
        (`self.Hit not Health Comp` HitResult)))))

(fn `Hit Healt Comp`
  (params (`Hit Result` :type "HitResult Structure (by ref)") (`Healt Comp` :type "PacHealthComponent Object Reference"))
  (bind (_hit_result_bblockinghit _hit_result_binitialoverlap _hit_result_time _hit_result_distance _hit_result_location) (`GameplayStatics.BreakHitResult` (`local.Hit Result`)))
  (`PacHealthComponent.TakeDamage` `Healt Comp` (`self.Damage Amount`) (`self.GetAvatarCharacter`))
  (`NiagaraFunctionLibrary.SpawnSystemAtLocation` (`self.ImpactDamage`) _hit_result_location (struct) (1.0 1.0 1.0) true true "AutoRelease" false))

(fn `Hit not Health Comp`
  (params (`hit Result` :type "HitResult Structure (by ref)"))
  (bind (_bblockinghit _binitialoverlap _time _distance _location _impactpoint _normal) (`GameplayStatics.BreakHitResult` `hit Result`))
  (bind _returnvalue (`KismetMathLibrary.RandomFloatInRange` 0.0 360.0))
  (bind (_decal_size_minmax_x _decal_size_minmax_y) (`KismetMathLibrary.BreakVector2D` (`self.Decal Size MinMax`)))
  (bind (_bblockinghit_2 _binitialoverlap_2 _time_2 _distance_2 _location_2 _impactpoint_2 _normal_2 _impactnormal) (`GameplayStatics.BreakHitResult` (`local.hit Result`)))
  (bind (_x _y _z) (`KismetMathLibrary.BreakRotIntoAxes` (`KismetMathLibrary.Conv_VectorToRotator` _impactnormal)))
  (`NiagaraFunctionLibrary.SpawnSystemAtLocation` (`self.ImpactGround`) _location (`KismetMathLibrary.MakeRotFromZ` _normal) (1.0 1.0 1.0) true true "AutoRelease" false)
  (`GameplayStatics.SpawnDecalAtLocation` (`self.Decal Material`) (`KismetMathLibrary.Conv_DoubleToVector` (`KismetMathLibrary.RandomFloatInRange` _decal_size_minmax_x _decal_size_minmax_y)) _location_2 (`KismetMathLibrary.MakeRotationFromAxes` _x (`KismetMathLibrary.RotateAngleAxis` _y _returnvalue _x) (`KismetMathLibrary.RotateAngleAxis` _z _returnvalue _x)) 10.0))