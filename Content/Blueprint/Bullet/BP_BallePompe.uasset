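; Pump-shotgun style bullet that instantly damages Pac characters in a cone along the shooter's aim, with a muzzle VFX.
; The cone is approximated by overlap spheres of growing radius and distance, then filtered by line traces back to the shooter that must hit a player character.
; Firing also pushes the shooter backward with root-motion recoil, and the bullet ends when that movement completes or fails.
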(event `self.K2_ActivateBullet`
  (bind _returnvalue (`self.GetAvatarCharacter`))
  (bind (_returnvalue_location _returnvalue_rotation) (`KismetMathLibrary.BreakTransform` (`self.GetTargetingTransform` _returnvalue)))
  (bind (_returnvalue_location_2 _returnvalue_rotation_2) (`KismetMathLibrary.BreakTransform` (`PacCharacter.GetFeedBackShootTransForm` _returnvalue)))
  (bind _returnvalue_2 (`KismetMathLibrary.GetForwardVector` _returnvalue_rotation))
  (`parent.OnTargetFound` (struct))
  (bind _newparam (`self.DetectActorInCone` (`Actor.K2_GetActorLocation` _returnvalue) _returnvalue_2))
  (cast `/Game/Blueprint/Character/BP_PacCharacter` _returnvalue)
  (`NiagaraFunctionLibrary.SpawnSystemAtLocation` (`self.Shoot VFX`) _returnvalue_location_2 _returnvalue_rotation_2)
  (`|ExecutionSequence`
    (:`then_0`
      (for _array_element _newparam
        (bind _aspac_character (cast `PacCharacter` _array_element))
        (`PacHealthComponent.TakeDamage` (`PacCharacter.HealthComponent` _aspac_character) (`self.Cone Damage `) (`self.GetAvatarCharacter`))))
    (:`then_1`
      (`AsyncRootMovement.AsyncRootMovement` (`Character.CharacterMovement` _returnvalue) (* _returnvalue_2 -1) (`self.RecoilStrength`) 0.25 false null "MaintainLastRootMotionVelocity"
        (:`OnComplete`
          _)
        (:`OnFail`
          _))
      (`self.K2_EndBullet`))))

(fn `DetectActorInCone`
  (params (StartLocation :type "Vector Structure") (ForwardVector :type "Vector Structure"))
  (returns (NewParam :type "Array of Actor Object Reference"))
  (locals (TargetFound :type "Array of Actor Object Reference") (ValidateTarget :type "Array of Actor Object Reference"))
  (bind _array (`|MakeArray` (`self.GetAvatarCharacter`) :!type "Actor Object Reference"))
  (for _index (range 1 (+ (`self.SphereNumber`) 1))
    (`KismetArrayLibrary.Array_Append` _array (`local.TargetFound`))
    (bind _returnvalue (* _index (`self.InitialRadius`)))
    (bind _outactors (`KismetSystemLibrary.SphereOverlapActors` (+ (* (`local.ForwardVector`) (* 2 _returnvalue)) (`local.StartLocation`)) (`KismetMathLibrary.Conv_IntToDouble` _returnvalue) (`self.Object Types`) "/Script/Pac.PacCharacter" _array))
    (for _array_element _outactors
      (`KismetArrayLibrary.Array_AddUnique` (`local.TargetFound`) _array_element)))
  (for _array_element_2 (`local.TargetFound`)
    (bind _outhit (`KismetSystemLibrary.LineTraceSingle` (`Actor.K2_GetActorLocation` _array_element_2) (`Actor.K2_GetActorLocation` (`self.GetAvatarCharacter`)) "TraceTypeQuery4" true (`local.TargetFound`) "None" false))
    (cast `PacPlayerCharacter` (`.HitActor` (`GameplayStatics.BreakHitResult` _outhit)))
    (`KismetArrayLibrary.Array_AddUnique` (`local.ValidateTarget`) _array_element_2))
  (return (`local.ValidateTarget`)))