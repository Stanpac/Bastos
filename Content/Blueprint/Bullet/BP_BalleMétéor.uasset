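; Meteor bullet Blueprint that explodes where it hits and deals area damage.
; On a blocking hit, after the parent logic, the blast radius scales with the impact's distance from the avatar character, clamped between limits.
; That radius sizes the explosion VFX and a sphere overlap, which damages actors with a PacHealthComponent, ignoring the avatar.
; An unconnected debug sphere draw remains in the graph.
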(event `self.OnTargetFound`
  (params (HitResult :type "HitResult Structure"))
  (bind _returnvalue (`self.GetAvatarCharacter`))
  (bind (_bblockinghit _binitialoverlap _time _distance _location) (`GameplayStatics.BreakHitResult` HitResult))
  (bind _returnvalue_2 (`KismetMathLibrary.FClamp` (* (`KismetMathLibrary.Vector_Distance` _location (`Actor.K2_GetActorLocation` _returnvalue)) (`self.RangeFactor`)) (`self.RangeMin`) (`self.RangeMax`)))
  (`parent.OnTargetFound` HitResult)
  (if _bblockinghit
    (bind _returnvalue_3 (`NiagaraFunctionLibrary.SpawnSystemAtLocation` (`self.Explosion VFX`) _location))
    (`NiagaraComponent.SetVariableFloat` _returnvalue_3 "AOE RANGE" (/ _returnvalue_2 50.0))
    (bind _outactors (`KismetSystemLibrary.SphereOverlapActors` _location _returnvalue_2 (`self.Object Types`) "/Script/Engine.Actor" (`|MakeArray` _returnvalue :!type "Actor Object Reference")))
    (for _array_element _outactors
      (bind _returnvalue_4 (`Actor.GetComponentByClass` _array_element "/Script/Pac.PacHealthComponent"))
      (`/Engine/EditorBlueprintResources/StandardMacros.IsValid` _returnvalue_4
        (:`Is Valid`
          (`PacHealthComponent.TakeDamage` _returnvalue_4 (`self.Explosion Damage`) (`self.GetAvatarCharacter`)))))))