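; BP_TPToLocation is a trigger actor that teleports the player to the location of a referenced actor, with zeroed rotation, when they overlap its box.
; Optional flags let it reset aggro on enemies listed by the game mode and restore the player's bullets from those saved in the game instance.
; A one-time-use flag makes it destroy itself afterwards.
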(event `self.Box.OnComponentBeginOverlap`
  (params (OverlappedComponent :type "PrimitiveComponent Object Reference") (OtherActor :type "Actor Object Reference") (OtherComp :type "PrimitiveComponent Object Reference") (OtherBodyIndex :type Integer) (bFromSweep :type Boolean) (SweepResult :type "HitResult Structure (by ref)"))
  (bind _aspac_player_character (cast `PacPlayerCharacter` OtherActor))
  (`self.K2_TeleportTo` :`self` _aspac_player_character :`DestLocation` (`self.K2_GetActorLocation` (`self.ActorToTp`)))
  (if (`self.ResetAggroEnemy?`)
    (bind _aspac_game_mode (cast `PacGameMode` (`GameplayStatics.GetGameMode`)))
    (for _array_element (`PacGameMode.GetEnemies` _aspac_game_mode)
      (bind _asbp_base_ennemy (cast `/Game/Blueprint/Ennemy/Enemy/BP_BaseEnnemy` _array_element))
      (`/Game/Blueprint/Ennemy/Enemy/BP_BaseEnnemy.Reset Aggro` _asbp_base_ennemy)
      (if (`self.GiveBackChargeur`) :!label _label
        (bind _aspac_game_instance (cast `PacGameInstance` (`GameplayStatics.GetGameInstance`)))
        (`PacBulletsComponent.SetNewBullets` (`PacCharacter.BulletsComponent` _aspac_player_character) (`PacGameInstance.GetSaveBullets` _aspac_game_instance)))
      (if (`self.OneTimeUse`)
        (`self.K2_DestroyActor`)))
    (else
      (goto _label))))

(fn `UserConstructionScript`)