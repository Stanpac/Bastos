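; Bullet pickup actor that gives its configured bullet class to a PacPlayerCharacter overlapping its sphere, placing it at the active bullet index of that character's BulletsComponent.
; Pickup plays a sound and, if OneTimeUse is set, disables collision and destroys the actor.
; The bullet's class defaults supply the text label at construction and the rotating mesh at BeginPlay.
; An invalid bullet class prints an error and expires the actor shortly after BeginPlay.
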(event `self.Sphere.OnComponentBeginOverlap`
  (params (OverlappedComponent :type "PrimitiveComponent Object Reference") (OtherActor :type "Actor Object Reference") (OtherComp :type "PrimitiveComponent Object Reference") (OtherBodyIndex :type Integer) (bFromSweep :type Boolean) (SweepResult :type "HitResult Structure (by ref)"))
  (bind _aspac_player_character (cast `PacPlayerCharacter` OtherActor))
  (bind _bulletscomponent (`PacCharacter.BulletsComponent` _aspac_player_character))
  (`PacBulletsComponent.AddBulletAt` _bulletscomponent (`PacBulletsComponent.GetActiveBulletIndex` _bulletscomponent) (`self.Bullet`))
  (`GameplayStatics.PlaySoundAtLocation` (`self.PickUpSound`) (`self.K2_GetActorLocation`) (struct) 1.0 1.0 0.0 null null null null)
  (if (`self.bOneTimeUse`)
    (`PrimitiveComponent.SetCollisionEnabled` (`self.Sphere`) "NoCollision")
    (`self.K2_DestroyActor`)))

(event `self.ReceiveBeginPlay`
  (bind _bullet (`self.Bullet`))
  (if (`KismetSystemLibrary.IsValidClass` _bullet)
    (`StaticMeshComponent.SetStaticMesh` (`self.StaticMesh`) (`.PickUpMesh` (defaults `Object` _bullet)))
    (`MovementComponent.SetUpdatedComponent` (`self.RotatingMovement`) (`self.StaticMesh`))
    (else
      (`KismetSystemLibrary.PrintString` "Class Not Valid for Bullet pick Up " true true (struct :`R` 1.0 :`B` 0.009947 :`A` 1.0) 5.0)
      (`self.SetLifeSpan` 0.1))))

(fn `UserConstructionScript`
  (`/Engine/EditorBlueprintResources/StandardMacros.IsValid` (`self.TextRender`)
    (:`Is Valid`
      (`TextRenderComponent.K2_SetText` (`self.TextRender`) (select `bool` (`KismetSystemLibrary.IsValidClass` (`self.Bullet`)) :`false` "None" :`true` (defaults `Object` (`self.Bullet`)))))))