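; BP_TPEndLevel is an end-of-level exit actor that returns the player to the lobby once the level is won.
; On BeginPlay it disables its Box collision and subscribes to the PacGameMode win event.
; Winning unhides the actor and enables query-only collision on the Box.
; A PacPlayerCharacter overlapping the Box then triggers SwitchToLobby on the PacGameInstance.
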(event `self.ReceiveBeginPlay`
  (bind _aspac_game_mode (cast `PacGameMode` (`GameplayStatics.GetGameMode`)))
  (add `PacGameMode.OnPlayerWinLevel` _aspac_game_mode (delegate `OnPlayerWinLevel_Event`))
  (`PrimitiveComponent.SetCollisionEnabled` (`self.Box`) "NoCollision"))

(event `OnPlayerWinLevel_Event`
  (`self.SetActorHiddenInGame` false)
  (`PrimitiveComponent.SetCollisionEnabled` (`self.Box`) "QueryOnly"))

(event `self.Box.OnComponentBeginOverlap`
  (params (OverlappedComponent :type "PrimitiveComponent Object Reference") (OtherActor :type "Actor Object Reference") (OtherComp :type "PrimitiveComponent Object Reference") (OtherBodyIndex :type Integer) (bFromSweep :type Boolean) (SweepResult :type "HitResult Structure (by ref)"))
  (cast `PacPlayerCharacter` OtherActor)
  (bind _aspac_game_instance (cast `PacGameInstance` (`GameplayStatics.GetGameInstance`)))
  (`PacGameInstance.SwitchToLobby` _aspac_game_instance))

(fn `UserConstructionScript`)