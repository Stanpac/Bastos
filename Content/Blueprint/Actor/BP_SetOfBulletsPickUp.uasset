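; Pickup actor that hands its configured set of bullet classes to the player character on overlap.
; A sphere overlap by a PacPlayerCharacter passes the bullets to its BulletsComponent through SetNewBullets and plays a pickup sound at the actor.
; When flagged one-time use, it then disables sphere collision and destroys itself.
; On BeginPlay it points RotatingMovement at the static mesh and removes invalid bullet classes while iterating the list.
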(event `self.Sphere.OnComponentBeginOverlap`
  (params (OverlappedComponent :type "PrimitiveComponent Object Reference") (OtherActor :type "Actor Object Reference") (OtherComp :type "PrimitiveComponent Object Reference") (OtherBodyIndex :type Integer) (bFromSweep :type Boolean) (SweepResult :type "HitResult Structure (by ref)"))
  (bind _aspac_player_character (cast `PacPlayerCharacter` OtherActor))
  (`PacBulletsComponent.SetNewBullets` (`PacCharacter.BulletsComponent` _aspac_player_character) (`self.Bullet`))
  (`GameplayStatics.PlaySoundAtLocation` (`self.PickUpSound`) (`self.K2_GetActorLocation`) (struct) 1.0 1.0 0.0 null null null null)
  (if (`self.bOneTimeUse`)
    (`PrimitiveComponent.SetCollisionEnabled` (`self.Sphere`) "NoCollision")
    (`self.K2_DestroyActor`)))

(event `self.ReceiveBeginPlay`
  (`MovementComponent.SetUpdatedComponent` (`self.RotatingMovement`) (`self.StaticMesh`))
  (for _array_element (`self.Bullet`)
    (if (not (`KismetSystemLibrary.IsValidClass` _array_element))
      (`KismetArrayLibrary.Array_RemoveItem` (`self.Bullet`) _array_element))))

(fn `UserConstructionScript`)