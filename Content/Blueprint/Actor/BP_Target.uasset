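; BP_Target is a target actor with a PacHealth component that sets health back to 5 whenever it hits zero.
; A sphere trigger shows its widget and sets PlayerInRange while a PacCharacter overlaps it, then reverses both on exit.
; Logic to push normalized health into the widget through SetLife is present but disconnected, so it never runs.
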(event `self.PacHealth.OnHealthChanged`
  (params (HealthComponent :type "PacHealthComponent Object Reference") (OldValue :type Integer) (NewValue :type Integer) (Instigator :type "Actor Object Reference"))
  (if (== (`KismetMathLibrary.Conv_IntToDouble` NewValue) 0.0)
    (`PacHealthComponent.SetHealth` (`self.PacHealth`) 5)))

(event `self.Sphere.OnComponentBeginOverlap`
  (params (OverlappedComponent :type "PrimitiveComponent Object Reference") (OtherActor :type "Actor Object Reference") (OtherComp :type "PrimitiveComponent Object Reference") (OtherBodyIndex :type Integer) (bFromSweep :type Boolean) (SweepResult :type "HitResult Structure (by ref)"))
  (if (`KismetMathLibrary.ClassIsChildOf` (`GameplayStatics.GetObjectClass` OtherActor) "/Script/Pac.PacCharacter")
    (set `self.PlayerInRange` true)
    (`SceneComponent.SetVisibility` (`self.Widget`) true false)))

(event `self.Sphere.OnComponentEndOverlap`
  (params (OverlappedComponent :type "PrimitiveComponent Object Reference") (OtherActor :type "Actor Object Reference") (OtherComp :type "PrimitiveComponent Object Reference") (OtherBodyIndex :type Integer))
  (if (`KismetMathLibrary.ClassIsChildOf` (`GameplayStatics.GetObjectClass` OtherActor) "/Script/Pac.PacCharacter")
    (set `self.PlayerInRange` false)
    (`SceneComponent.SetVisibility` (`self.Widget`) false false)))

(fn `UserConstructionScript`)