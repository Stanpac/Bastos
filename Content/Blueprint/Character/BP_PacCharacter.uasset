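; First-person player character with coyote time, sprint FOV effects, fire and reload montages, rail grinding, and health-driven damage and death handling.
; While airborne, a looping timer sphere-traces for BP_splines, then sets Flying mode and picks direction from camera facing versus spline tangent.
; Tick moves the character along the spline until a forward trace misses, then root motion launches it off.
; Damage grants temporary immunity; death's end returns to the menu.
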(event `self.ReceiveBeginPlay`
  (bind _asplayer_controller (cast `PlayerController` (`self.GetController`)))
  (bind _returnvalue (`|CreateWidget` "/Game/UI/Character/W_PlayerWidget.W_PlayerWidget_C" _asplayer_controller))
  (bind _output_get (set `self.PlayerWidget` _returnvalue))
  (`UserWidget.AddToPlayerScreen` _output_get 0)
  (`/Game/UI/Character/W_PlayerWidget.InitLife` _returnvalue (`PacHealthComponent.GetHealth` (`self.HealthComponent`))))

(event `self.ReceiveTick`
  (params (DeltaSeconds :type "Float (single-precision)"))
  (`self.CheckRailMovement` DeltaSeconds))

(event `self.OnLanded`
  (params (Hit :type "HitResult Structure (by ref)"))
  ;[0 0.5557 0.9688 0.5] On Land
  ;;[0.15 0 0 0.5] TO SET
  (`GameplayStatics.PlaySound2D` null 1.0 1.0 0.0 null null false)
  (`GameplayStatics.PlayWorldCameraShake` "/Game/Blueprint/Camera/CameraShake/BP_CS_Land.BP_CS_Land_C" (`self.K2_GetActorLocation`) 0.0 500.0)
  (set `CharacterMovementComponent.FallingLateralFriction` 8.0 (`self.CharacterMovement`))
  (`GameplayTagCountContainerInterface.UpdateTagCount` (struct :`TagName` "Gameplay.CoyoteTime") -10))

(event `self.OnWalkingOffLedge`
  (params (PreviousFloorImpactNormal :type "Vector Structure (by ref)") (PreviousFloorContactNormal :type "Vector Structure (by ref)") (PreviousLocation :type "Vector Structure (by ref)") (TimeDelta :type "Float (single-precision)"))
  ;[0 0.5488 1 0.5] Coyote Time
  (`GameplayTagCountContainerInterface.UpdateTagCount` (struct :`TagName` "Gameplay.CoyoteTime") 1)
  (`KismetSystemLibrary.RetriggerableDelay` (`self.CoyoteTime`))
  (`GameplayTagCountContainerInterface.UpdateTagCount` (struct :`TagName` "Gameplay.CoyoteTime") -10))

(event `RailJump`
  (params (`Ejected?` :type Boolean :default true))
  ;[1 1 1 0.5] Rail
  ;;[0 0.5557 0.9688 0.5] Rail Jump
  (`ActorComponent.Deactivate` (`self.NS_Speedlines`))
  (`AudioComponent.Stop` (`self.RailSound`))
  (`GameplayStatics.PlaySoundAtLocation` "/Game/SoundDesign/Walking/Rail/RailMovementEnd.RailMovementEnd" (`SceneComponent.K2_GetComponentLocation` (`self.RailSound`)) (struct) 1.0 1.0 0.0 null null null null)
  (`CharacterMovementComponent.SetMovementMode` (`self.CharacterMovement`) "MOVE_Falling" 0)
  (set `self.bOnSpline` false)
  (`AsyncRootMovement.AsyncRootMovement` (`self.CharacterMovement`) (+ (* (`self.GetActorForwardVector`) 2.0) (* (`self.GetActorUpVector`) (select `bool` `Ejected?` :`false` 2.0 :`true` 1.0))) (`self.LaunchForce`) 0.25 true null "MaintainLastRootMotionVelocity"
    (:`then`
      (`KismetSystemLibrary.Delay` 0.2)
      (`self.StartTrace`))))

(event `self.OnJumped`
  ;[0 0.5557 0.9688 0.5] On Jump
  (`parent.OnJumped`)
  (`GameplayTagCountContainerInterface.UpdateTagCount` (struct :`TagName` "Gameplay.CoyoteTime") -10)
  (`GameplayStatics.PlayWorldCameraShake` "/Game/Blueprint/Camera/CameraShake/BP_CS_Jump.BP_CS_Jump_C" (`self.K2_GetActorLocation`) 0.0 500.0)
  (if (not (`self.bOnSpline`))
    (`self.StartTrace`)))

(event `StartTrace`
  ;[1 1 1 0.5] Rail
  ;;[0 0.5557 0.9688 0.5] Start Trace
  (if (not (`KismetSystemLibrary.K2_IsTimerActiveHandle` (`self.TraceTimer`)))
    (bind _returnvalue (`KismetSystemLibrary.K2_SetTimerDelegate` (`|CreateDelegate` :!event `SplineTrace`) 0.1 true))
    (set `self.TraceTimer` _returnvalue)))

(event `StopTrace`
  ;[1 1 1 0.5] Rail
  ;;[0 0.5557 0.9688 0.5] Stop Trace
  (`KismetSystemLibrary.K2_ClearAndInvalidateTimerHandle` (`self.TraceTimer`)))

(event `self.K2_Sprint`
  ;[0 0.5557 0.9688 0.5] Sprint
  (if (> (`KismetMathLibrary.VSizeXY` (`MovementComponent.Velocity` (`self.CharacterMovement`))) 0.0)
    (`ActorComponent.Activate` (`self.NS_Speedlines`) true)
    ;;[0.15 0 0 0.5] TO SET
    (`GameplayStatics.PlaySound2D` null 1.0 1.0 0.0 null null false)
    (bind (_direction _alpha) (`Timeline|ChangeFov` :!label _label)
      (:`Update`
        (`CameraComponent.SetFieldOfView` (`self.CameraComponent`) (`KismetMathLibrary.Lerp` (`self.WalkFov`) (`self.SprintFov`) _alpha))))))

(event `self.K2_StopSprint`
  ;[0 0.5557 0.9688 0.5] Sprint
  (`ActorComponent.Deactivate` (`self.NS_Speedlines`))
  (goto _label :!via `Reverse`))

(event `SplineTrace`
  (bind _grindrail (`self.GrindRail`))
  (bind _returnvalue (- (`self.K2_GetActorLocation`) (`KismetMathLibrary.MakeVector` 0.0 0.0 (`CapsuleComponent.CapsuleHalfHeight` (`self.CapsuleComponent`)))))
  ;[1 1 1 0.5] Rail
  ;;[0 0.5557 0.9688 0.5] SplineTrace
  (if (`NavMovementComponent.IsFalling` (`self.CharacterMovement`))
    (bind (_outhit _returnvalue_2) (`KismetSystemLibrary.SphereTraceSingle` _returnvalue _returnvalue 40.0 "TraceTypeQuery3"))
    (if _returnvalue_2
      (bind (_bblockinghit _binitialoverlap _time _distance _location _impactpoint _normal _impactnormal _physmat _hitactor) (`GameplayStatics.BreakHitResult` _outhit))
      (`KismetSystemLibrary.IsObjectOfSoftClass` _hitactor "/Game/Blueprint/Ramp/BP_splines.BP_splines_C"
        (:`True`
          (bind _asbp_splines (cast `/Game/Blueprint/Ramp/BP_splines` _hitactor))
          (set `self.GrindRail` _asbp_splines)
          (`MovementComponent.StopMovementImmediately` (`self.CharacterMovement`))
          (`CharacterMovementComponent.SetMovementMode` (`self.CharacterMovement`) "MOVE_Flying" 0)
          (`self.StopTrace`)
          (bind _distance_2 (`self.Find Spline Distance at Overlap` _impactpoint _grindrail))
          (bind _output_get (set `self.Distance` _distance_2))
          (`self.DefineRailDirection` _grindrail _output_get)
          (set `self.bOnSpline` true)
          (`ActorComponent.Activate` (`self.NS_Speedlines`) false)
          (`AudioComponent.Play` (`self.RailSound`) 0.0))))))

(event `self.K2_Fire`
  ;[0.9271 0.4884 0 0.5] Fire
  (`|PlayMontage` (`self.FirsPersonMesh`) (`self.FireMontage`)
    (:`then`
      (`self.StopSprint`))
    (:`OnCompleted`
      (if (and (`self.bUseShootingAnimationTime`) (`GameplayTagAssetInterface.HasAllMatchingGameplayTags` (`BlueprintGameplayTagLibrary.MakeLiteralGameplayTagContainer` (struct :`GameplayTags` (struct :`(TagName` "Gameplay.PreventFromShooting")))))) :!label _label_2
        (`self.OnFireTimerExpired`)))
    (:`OnInterrupted`
      (goto _label_2))))

(event `CheckRailMovement`
  (params (DeltaTime :type "Float (double-precision)"))
  (bind _spline (`/Game/Blueprint/Ramp/BP_splines.Spline` (`self.GrindRail`)))
  (bind _returnvalue (`SplineComponent.GetDirectionAtDistanceAlongSpline` _spline (`self.Distance`) "Local"))
  (bind _returnvalue_2 (+ (- (`self.K2_GetActorLocation`) (`KismetMathLibrary.MakeVector` 0.0 0.0 (`CapsuleComponent.CapsuleHalfHeight` (`self.CapsuleComponent`)))) (* (`self.GetActorForwardVector`) 50.0)))
  ;[1 1 1 0.5] Rail
  ;;[0 0.5557 0.9688 0.5] MoveOn Rail
  (if (`self.bOnSpline`)
    (`/Engine/EditorBlueprintResources/StandardMacros.IsValid` (`self.GrindRail`)
      (:`Is Valid`
        (set `self.Distance` (+ (`self.Distance`) (* DeltaTime (select `bool` (`self.bInverseDirection`) :`false` (`self.SpeedOnSpline`) :`true` (* (`self.SpeedOnSpline`) -1.0)))))
        (`self.K2_SetActorLocationAndRotation` (+ (* (`self.GetActorUpVector`) (`CapsuleComponent.CapsuleHalfHeight` (`self.CapsuleComponent`))) (`SplineComponent.GetLocationAtDistanceAlongSpline` _spline (`self.Distance`) "World")) (`KismetMathLibrary.Conv_VectorToRotator` (select `bool` (`self.bInverseDirection`) :`false` _returnvalue :`true` (* _returnvalue -1.0))))
        (bind (_outhit _returnvalue_3) (`KismetSystemLibrary.SphereTraceSingle` :`Start` _returnvalue_2 :`End` _returnvalue_2 :`Radius` 25.0 :`TraceChannel` "TraceTypeQuery3" :`TraceColor` (struct :`R` 1.0 :`B` 0.854139 :`A` 1.0) :`TraceHitColor` (struct :`G` 0.14433 :`B` 1.0 :`A` 1.0)))
        (if (not _returnvalue_3)
          (`self.RailJump` true))))))

(event `self.K2_Reload`
  ;[0.9271 0.4884 0 0.5] Reload
  (`|PlayMontage` (`self.FirsPersonMesh`) (`self.ReloadMontage`)
    (:`OnCompleted`
      _)
    (:`OnInterrupted`
      _))
  (if (and (`self.bUseReloadAnimationTime`) (`GameplayTagAssetInterface.HasAllMatchingGameplayTags` (`BlueprintGameplayTagLibrary.MakeLiteralGameplayTagContainer` (struct :`GameplayTags` (struct :`(TagName` "Gameplay.PreventFromReloading") :`(TagName` "Gameplay.PreventFromShooting"))))))
    (`self.OnReloadTimerExpired`)))

(event `self.HealthComponent.OnTakeDamage`
  (params (HealthComponent :type "PacHealthComponent Object Reference") (OldValue :type Integer) (NewValue :type Integer) (Instigator :type "Actor Object Reference"))
  ;[0.1501 1 0.01349 0.5] Take Damage
  (`PacEffectComponent.TryAddOrUpdateEffect` (`self.EffectComponent`) "/Game/Blueprint/Effects/BP_DamageImmunityEffect.BP_DamageImmunityEffect_C" 1)
  (`GameplayStatics.PlaySound2D` "/Game/SoundDesign/Damaged/Hit_Input.Hit_Input" 1.0 1.0 0.0 null null false))

(event `EnhancedInput|/Game/Blueprint/Input/InputAction/IA_Jump`
  (params (ActionValue :type Boolean) (ElapsedSeconds :type "Float (double-precision)") (TriggeredSeconds :type "Float (double-precision)") (InputAction :type "InputAction Object Reference" :default "/Game/Blueprint/Input/InputAction/IA_Jump.IA_Jump"))
  (:`Triggered`
    (if (`self.bOnSpline`)
      _)))

(event `self.K2_OnEndDeath`
  (bind _playerwidget (`self.PlayerWidget`))
  ;[0.1501 1 0.01349 0.5] Death
  (`/Engine/EditorBlueprintResources/StandardMacros.IsValid` _playerwidget
    (:`Is Valid`
      (`Widget.RemoveFromParent` _playerwidget)
      (bind _aspac_game_instance (cast `PacGameInstance` (`GameplayStatics.GetGameInstance`)))
      (`PacGameInstance.OpenMenuLevel` _aspac_game_instance))))

(event `self.HealthComponent.OnDeath`
  ;[0.15 0 0 0.5] TO SET
  (`GameplayStatics.PlaySound2D` "/Game/SoundDesign/Damaged/Death_Input.Death_Input" 1.0 1.0 0.0 null null))

(fn `DefineRailDirection`
  (params (Spline :type "/Game/Blueprint/Ramp/BP_splines Object Reference (by ref)") (Distance :type "Float (double-precision) (by ref)"))
  (if (< (`KismetMathLibrary.Dot_VectorVector` (`SplineComponent.GetTangentAtDistanceAlongSpline` (`/Game/Blueprint/Ramp/BP_splines.Spline` Spline) Distance "Local") (`SceneComponent.GetForwardVector` (`self.CameraComponent`))) 0.0)
    (set `self.bInverseDirection` true)
    (else
      (set `self.bInverseDirection` false))))

(fn `Find Spline Distance at Overlap`
  (params (Location :type "Vector Structure") (Spline :type "/Game/Blueprint/Ramp/BP_splines Object Reference (by ref)"))
  (returns (Distance :type "Float (double-precision)"))
  (bind _returnvalue (`SplineComponent.FindInputKeyClosestToWorldLocation` (`/Game/Blueprint/Ramp/BP_splines.Spline` Spline) Location))
  (bind _spline (`/Game/Blueprint/Ramp/BP_splines.Spline` (`local.Spline`)))
  (bind _returnvalue_2 (`KismetMathLibrary.FTrunc` _returnvalue))
  (bind _returnvalue_3 (`SplineComponent.GetDistanceAlongSplineAtSplinePoint` _spline (`KismetMathLibrary.FTrunc` _returnvalue)))
  (return (+ _returnvalue_3 (* (- (`SplineComponent.GetDistanceAlongSplineAtSplinePoint` _spline (+ _returnvalue_2 1)) _returnvalue_3) (- _returnvalue _returnvalue_2)))))

(fn `UserConstructionScript`)